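; Default player controller for the truck game, managing loading screen, root HUD and dialogue UI in drive mode or on foot.
; In drive mode, menu selections blend cameras and start named dialogue knots, whose events start auto or manual driving by swapping Enhanced Input contexts, return the view, or load the main menu.
; Tick feeds truck telemetry to the HUD, and helpers switch pawn UI and transition the sky's time of day.
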(event Custom|OnEnterDrivingMode_Event
  (CallFunction|ChangeMappingContext "/Game/Dynamic/Vehicle/Input/IMC_Vehicle.IMC_Vehicle" "/Game/Dynamic/Vehicle/Input/IMC_Vehicle_ManualDrive.IMC_Vehicle_ManualDrive" 20)
  (Default|StartManualDrive (Variables|Vehicle|GetTruck_Ref))
  (Utilities|FlowControl|Delay 0.2)
  (Variables|/Game/Dynamic/Vehicle/peterbilt-379/BP_Peterbilt379_3.BP_Peterbilt379_3_C|SetIsDriveEnabled (Variables|Vehicle|GetTruck_Ref) true)
  (UI|BacktoTruckView (Variables|UI|GetDialogueUI) 0.5))

(event Custom|OnLoadingCompleted
  ;[0.15 0.15 0.15 0.5] 데모로 돌아가기
  (Variables|/Game/Dynamic/UI/WBP_LoadingScreen.WBP_LoadingScreen_C|SetCurrentLoadingDuration (stale Custom|OpenMainMenuAfterLoading _loadingscreenref) (Variables|/Game/Dynamic/UI/WBP_LoadingScreen.WBP_LoadingScreen_C|GetLoadingDuration (stale Custom|OpenMainMenuAfterLoading _loadingscreenref)))
  (Utilities|FlowControl|Delay 1.0)
  (Game|OpenLevel(byObjectReference) "/Game/Dynamic/Scenes/Mainmenu.Mainmenu"))

(event Custom|ChangeViewEvent
  (params (Selection :type Enum_TrailerCam%20Enum :default "NewEnumerator3"))
  (bind _dialogueui (Variables|UI|GetDialogueUI))
  (bind _dialogueui_2 (Variables|UI|GetDialogueUI))
  ;[0.15 0.15 0.15 0.5] 3D Widget Interaction
  (bind _output_get (Vehicle|GetTrailerRef))
  (Default|SetViewTargetCameraTransform _output_get Selection 0.5)
  (switch Utilities|FlowControl|Switch|SwitchonEnum_TrailerCam Selection
    (:NewEnumerator3
      (Variables|UI|SetButtonSelection "NewEnumerator1")
      (Variables|UI|SetInKnotName "Marie"))
    (:NewEnumerator0
      (Variables|UI|SetButtonSelection "NewEnumerator2")
      (Variables|UI|SetInKnotName "Cargo")))
  ;[0.15 0.15 0.15 0.5] Dialogue Widget 이름 설정
  (Widget|SetVisibility (Variables|UI|GetRootUI) "Hidden")
  (UI|AddDialogueUI (Variables|UI|GetDialogueUI) (Variables|UI|GetInKnotName))
  (switch Utilities|FlowControl|Switch|SwitchonEnum_ButtonTexture (Variables|UI|GetButtonSelection)
    (:NewEnumerator0
      ;[0.15 0.15 0.15 0.5] 차량 수리 완료
      (EventDispatchers|UnbindallEventsfromOnVehicleRepaired _dialogueui)
      (EventDispatchers|BindEventtoOnVehicleRepaired _dialogueui (delegate Custom|StartDrive))
      ;[0.15 0.15 0.15 0.5] 수동운전 선택
      (EventDispatchers|AssignOnEnterDrivingMode (Variables|UI|GetDialogueUI) (delegate Custom|OnEnterDrivingMode_Event)))
    (:NewEnumerator1
      _)
    (:NewEnumerator2
      _))
  ;[0.15 0.15 0.15 0.5] 돌아가기
  (EventDispatchers|UnbindallEventsfromOnDialogueFinished _dialogueui_2)
  (EventDispatchers|BindEventtoOnDialogueFinished _dialogueui_2 (delegate Custom|ChangeToMainCamEvent))
  ;[0.15 0.15 0.15 0.5] 데모로 돌아가기
  (EventDispatchers|BindEventtoOnDemoEnd (Variables|UI|GetDialogueUI) (delegate Custom|OpenMainMenuAfterLoading)))

(event Custom|StartDrive
  (CallFunction|ChangeMappingContext "/Game/Dynamic/Vehicle/Input/IMC_Vehicle_ManualDrive.IMC_Vehicle_ManualDrive" "/Game/Dynamic/Vehicle/Input/IMC_Vehicle.IMC_Vehicle" 10)
  (Default|StartAutoDrive (Variables|Vehicle|GetTruck_Ref))
  (Variables|/Game/Dynamic/Vehicle/peterbilt-379/BP_Peterbilt379_3.BP_Peterbilt379_3_C|SetIsDriveEnabled (Variables|Vehicle|GetTruck_Ref) true)
  (UI|BacktoTruckView (Variables|UI|GetDialogueUI) 0.5))

(event Custom|OpenMainMenuAfterLoading
  ;[0.15 0.15 0.15 0.5] 데모로 돌아가기
  (bind _loadingscreenref (UI|ShowLoadingScreen (Variables|Default|GetLoading%20Duration)))
  (EventDispatchers|BindEventtoOnLoadingCompleted _loadingscreenref (delegate Custom|OnLoadingCompleted)))

(event Custom|GameStart
  (bind _rootui (Variables|UI|GetRootUI))
  (bind _loadingscreen_ref (Variables|UI|GetLoadingScreen_Ref))
  (Default|SetAllVisible (Variables|/Game/Dynamic/Vehicle/peterbilt-379/BP_Peterbilt379_3.BP_Peterbilt379_3_C|GetFloatingButton (Variables|Vehicle|GetTruck_Ref)) "Collapsed")
  (Variables|/Game/Dynamic/UI/WBP_LoadingScreen.WBP_LoadingScreen_C|SetCurrentLoadingDuration _loadingscreen_ref (Variables|/Game/Dynamic/UI/WBP_LoadingScreen.WBP_LoadingScreen_C|GetLoadingDuration _loadingscreen_ref))
  (Utilities|FlowControl|Delay 1.0)
  (Widget|RemovefromParent _loadingscreen_ref)
  (Variables|Default|SetbShowMouseCursor true)
  (if (Variables|Default|GetIsFirstGame)
    (EventDispatchers|BindEventtoOnDialogueFinished (Variables|UI|GetDialogueUI) (delegate Custom|OnDialogueFinished))
    (else
      (UserInterface|Viewport|AddtoViewport _rootui 0)
      (Class|WidgetSwitcher|SetActiveWidgetIndex (Variables|/Game/Dynamic/UI/WBP_RootUI.WBP_RootUI_C|GetWidgetSwitcher_Pawn _rootui) 1)
      (Variables|Default|SetbShowMouseCursor true)
      (Input|SetInputModeGameandUI (Game|GetPlayerController 0) 0 "DoNotLock" false false))))

(event Custom|DriveEvent
  (bind _dialogueui (Variables|UI|GetDialogueUI))
  (bind _dialogueui_2 (Variables|UI|GetDialogueUI))
  ;[0.15 0.15 0.15 0.5] 3D Widget Interaction
  (Default|ChangeCamViewDriveSelected (Variables|Vehicle|GetTruck_Ref))
  (Variables|UI|SetButtonSelection "NewEnumerator0")
  (Variables|UI|SetInKnotName "Nyx")
  ;[0.15 0.15 0.15 0.5] Dialogue Widget 이름 설정
  (Widget|SetVisibility (Variables|UI|GetRootUI) "Hidden")
  (UI|AddDialogueUI (Variables|UI|GetDialogueUI) (Variables|UI|GetInKnotName))
  (switch Utilities|FlowControl|Switch|SwitchonEnum_ButtonTexture (Variables|UI|GetButtonSelection)
    (:NewEnumerator0
      ;[0.15 0.15 0.15 0.5] 차량 수리 완료
      (EventDispatchers|UnbindallEventsfromOnVehicleRepaired _dialogueui)
      (EventDispatchers|BindEventtoOnVehicleRepaired _dialogueui (delegate Custom|StartDrive))
      ;[0.15 0.15 0.15 0.5] 수동운전 선택
      (EventDispatchers|AssignOnEnterDrivingMode (Variables|UI|GetDialogueUI) (delegate Custom|OnEnterDrivingMode_Event)))
    (:NewEnumerator1
      _)
    (:NewEnumerator2
      _))
  ;[0.15 0.15 0.15 0.5] 돌아가기
  (EventDispatchers|UnbindallEventsfromOnDialogueFinished _dialogueui_2)
  (EventDispatchers|BindEventtoOnDialogueFinished _dialogueui_2 (delegate Custom|ChangeToMainCamEvent))
  ;[0.15 0.15 0.15 0.5] 데모로 돌아가기
  (EventDispatchers|BindEventtoOnDemoEnd (Variables|UI|GetDialogueUI) (delegate Custom|OpenMainMenuAfterLoading)))

(event Custom|ChangeToMainCamEvent
  ;[0.15 0.15 0.15 0.5] 돌아가기
  (UI|BacktoTruckView (Variables|UI|GetDialogueUI) 0.5)
  (Default|CallOnBacktoMainCam))

(event Custom|OnDialogueFinished
  (bind _rootui (Variables|UI|GetRootUI))
  (Default|SetAllVisible (Variables|/Game/Dynamic/Vehicle/peterbilt-379/BP_Peterbilt379_3.BP_Peterbilt379_3_C|GetFloatingButton (Variables|Vehicle|GetTruck_Ref)) "Visible")
  (Variables|Default|SetIsFirstGame false)
  (Widget|RemovefromParent (Variables|UI|GetDialogueUI))
  (UserInterface|Viewport|AddtoViewport _rootui 0)
  (Class|WidgetSwitcher|SetActiveWidgetIndex (Variables|/Game/Dynamic/UI/WBP_RootUI.WBP_RootUI_C|GetWidgetSwitcher_Pawn _rootui) 1)
  (Variables|Default|SetbShowMouseCursor true)
  (Input|SetInputModeGameandUI (Game|GetPlayerController 0) 0 "DoNotLock" false false))

(event EventBeginPlay
  (UI|ShowLoadingScreen 3.5)
  (bind _returnvalue (Actor|GetActorOfClass "/Game/Dynamic/Blueprints/Sky/BP_DynamicSky_v2.BP_DynamicSky_v2_C"))
  (Variables|Default|SetDynamicSky_Ref _returnvalue)
  (Utilities|Casting|CastToGM_DriveMode (Game|GetGameMode)
    (:then
      (Variables|Default|SetIsDirveGM true)
      (bind _asbp_peterbilt_379_3 (Utilities|Casting|CastToBP_Peterbilt379_3 (Game|Player|GetPlayerPawn 0)))
      (Variables|Vehicle|SetTruck_Ref _asbp_peterbilt_379_3)
      (bind _returnvalue_2 (UserInterface|CreateWidget "/Game/Dynamic/UI/WBP_RootUI.WBP_RootUI_C"))
      (Variables|UI|SetRootUI _returnvalue_2)
      (bind _returnvalue_3 (UserInterface|CreateWidget "/Game/Dynamic/UI/DialogueUI/WBP_Dialogue.WBP_Dialogue_C"))
      (Variables|UI|SetDialogueUI _returnvalue_3)
      (if (Variables|Default|GetIsFirstGame)
        (UI|AddDialogueUI (Variables|UI|GetDialogueUI) "Bootup")
        (EventDispatchers|BindEventtoOnReadytoPlay (Variables|Vehicle|GetTruck_Ref) (delegate Custom|GameStart))
        (else
          (EventDispatchers|BindEventtoOnReadytoPlay (Variables|Vehicle|GetTruck_Ref) (delegate Custom|GameStart)))))
    (:CastFailed
      (bind _returnvalue_4 (UserInterface|CreateWidget "/Game/Dynamic/UI/WBP_RootUI.WBP_RootUI_C"))
      (bind _output_get (Variables|UI|SetRootUI _returnvalue_4))
      (UserInterface|Viewport|AddtoViewport _output_get 0)
      (bind _asbp_player (Utilities|Casting|CastToBP_Player (Game|Player|GetPlayerPawn 0)))
      (Variables|Default|SetCharacter_Ref _asbp_player))))

(event EventTick
  (params (DeltaSeconds :type Float%20%28single-precision%29))
  (bind _truck_ref (Variables|Vehicle|GetTruck_Ref))
  (bind _truck_ref_2 (Variables|Vehicle|GetTruck_Ref))
  (bind _truck_ref_3 (Variables|Vehicle|GetTruck_Ref))
  (bind _rootui (Variables|UI|GetRootUI))
  (bind _vehiclemovementcomponent (Variables|/Script/ChaosVehicles.WheeledVehiclePawn|GetVehicleMovementComponent _truck_ref))
  (bind _vehiclemovementcomponent_2 (Variables|/Script/ChaosVehicles.WheeledVehiclePawn|GetVehicleMovementComponent _truck_ref_3))
  (if (Variables|Default|GetIsDirveGM)
    ;[0.15 0.15 0.15 0.5] 차량 주행 중에만 사용
    (Default|UpdateSpeed _rootui (Vehicle|GetForwardSpeed _vehiclemovementcomponent_2) :!label _label)
    (Default|UpdateGear _rootui (Class|ChaosVehicleMovementComponent|GetCurrentGear _vehiclemovementcomponent_2))
    (bind _totaldistance (Default|GetTotalDistanceKm (Variables|Vehicle|GetTruck_Ref)))
    (Default|UpdateTotalDistance _rootui _totaldistance)
    (Default|UpdateCompass _rootui (- 3.6e+02 (.yaw (Transformation|GetActorRotation (Variables|Vehicle|GetTruck_Ref)))))
    (Default|CheckAutoDrive _rootui (Variables|/Game/Dynamic/Vehicle/peterbilt-379/BP_Peterbilt379_3.BP_Peterbilt379_3_C|GetIsDriveEnabled _truck_ref_2) (Variables|/Game/Dynamic/Vehicle/peterbilt-379/BP_Peterbilt379_3.BP_Peterbilt379_3_C|GetIsAuto _truck_ref_2))
    (Default|CheckTransimmision _rootui (Class|ChaosVehicleMovementComponent|GetUseAutoGears _vehiclemovementcomponent))
    (bind _aschaos_wheeled_vehicle_movement_component (Utilities|Casting|CastToChaosWheeledVehicleMovementComponent _vehiclemovementcomponent))
    (Default|Rppm _rootui (Class|ChaosWheeledVehicleMovementComponent|GetEngineRotationSpeed _aschaos_wheeled_vehicle_movement_component))
    (elif (Variables|/Game/Dynamic/Character/BP_Player.BP_Player_C|GetInCar (Variables|Default|GetCharacter_Ref))
      (goto _label))))

(event Input|KeyboardEvents|Escape
  (params (Key :type Key%20Structure :default "None"))
  (:Pressed
    (Default|CallPasueUI (Variables|UI|GetRootUI))))

(fn ConstructionScript)

(fn ShowLoadingScreen
  (params (LoadingDuration :type Float%20%28double-precision%29))
  (Utilities|IsValid (Variables|UI|GetLoadingScreen_Ref)
    (:Is%20Valid
      (Variables|/Game/Dynamic/UI/WBP_LoadingScreen.WBP_LoadingScreen_C|SetCurrentLoadingDuration (Variables|UI|GetLoadingScreen_Ref) 0.0))
    (:Is%20Not%20Valid
      ;[0.15 0.15 0.15 0.5] 처음 level 진입시
      (bind _returnvalue (UserInterface|CreateWidget "/Game/Dynamic/UI/WBP_LoadingScreen.WBP_LoadingScreen_C" 0 (* LoadingDuration 0.5) LoadingDuration))
      (Variables|UI|SetLoadingScreen_Ref _returnvalue)))
  (UserInterface|Viewport|AddtoViewport (Variables|UI|GetLoadingScreen_Ref) 100)
  (Variables|Default|SetbShowMouseCursor false)
  (Input|SetInputModeUIOnly (Game|GetPlayerController 0) (Variables|UI|GetLoadingScreen_Ref) "DoNotLock" false)
  (return (Variables|UI|GetLoadingScreen_Ref)))

(fn ShowVehicleUI
  (Class|WidgetSwitcher|SetActiveWidgetIndex (Variables|/Game/Dynamic/UI/WBP_RootUI.WBP_RootUI_C|GetWidgetSwitcher_Pawn (Variables|UI|GetRootUI)) 1)
  (bind _asbp_peterbilt_379_3 (Utilities|Casting|CastToBP_Peterbilt379_3 (Game|Player|GetPlayerPawn 0)))
  (Variables|Vehicle|SetTruck_Ref _asbp_peterbilt_379_3))

(fn ShowCharacterUI
  (Class|WidgetSwitcher|SetActiveWidgetIndex (Variables|/Game/Dynamic/UI/WBP_RootUI.WBP_RootUI_C|GetWidgetSwitcher_Pawn (Variables|UI|GetRootUI))))

(fn GetTrailerRef
  (Utilities|IsValid (Variables|Vehicle|GetTrailer_Ref)
    (:Is%20Valid
      (return (Variables|Vehicle|GetTrailer_Ref)))
    (:Is%20Not%20Valid
      (bind _returnvalue (Actor|GetActorOfClass "/Game/Dynamic/Vehicle/Truck_Trailer/BP_Truck_Trailer.BP_Truck_Trailer_C"))
      (Utilities|IsValid _returnvalue
        (:Is%20Valid
          (Variables|Vehicle|SetTrailer_Ref _returnvalue)
          (return (Variables|Vehicle|GetTrailer_Ref)))
        (:Is%20Not%20Valid
          (Development|PrintString "Fail"))))))

(fn BacktoTruckView
  (params (WidgetToRemove :type Widget%20Object%20Reference) (BlendTime :type Float%20%28single-precision%29))
  (Widget|RemovefromParent WidgetToRemove)
  (Widget|SetVisibility (Variables|UI|GetRootUI) "SelfHitTestInvisible")
  (Input|SetInputModeGameandUI (Game|GetPlayerController 0) 0 "DoNotLock" false false)
  (Default|SetViewTargetCamera (Variables|Vehicle|GetTruck_Ref) BlendTime))

(fn AddDialogueUI
  (params (DialogueUI :type WBP%20Dialogue%20Object%20Reference) (InKnotName :type String))
  (UserInterface|Viewport|AddtoViewport DialogueUI 10)
  (Input|SetInputModeUIOnly (Game|GetPlayerController 0) 0 "DoNotLock" false)
  (Default|Startfrom DialogueUI InKnotName))

(fn TransitTime
  (params (TargetTime :type Float%20%28double-precision%29) (Duration :type Float%20%28double-precision%29))
  (Default|TransitiontoTimeOfDay (Variables|Default|GetDynamicSky_Ref) TargetTime Duration))

(fn GetDynamicSkyRef
  (return (Variables|Default|GetDynamicSky_Ref)))

(fn ChangeMappingContext
  (params (MappingContextToRemove :type Input%20Mapping%20Context%20Object%20Reference) (MappingContextToAdd :type Input%20Mapping%20Context%20Object%20Reference) (Priority :type Integer))
  (bind _returnvalue (Game|GetPlayerController 0))
  (bind _returnvalue_2 (PlayerController|LocalPlayerSubsystems|GetEnhancedInputLocalPlayerSubsystem _returnvalue))
  (Input|RemoveMappingContext _returnvalue_2 MappingContextToRemove "(bIgnoreAllPressedKeysUntilRelease=True,bForceImmediately=False,bNotifyUserSettings=False)")
  (Input|AddMappingContext _returnvalue_2 MappingContextToAdd Priority "(bIgnoreAllPressedKeysUntilRelease=True,bForceImmediately=False,bNotifyUserSettings=False)"))