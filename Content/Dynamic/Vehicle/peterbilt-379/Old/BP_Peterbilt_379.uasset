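; Drivable Peterbilt 379 truck pawn with Enhanced Input driving, a rotatable spring-arm camera and a toggleable autodrive.
; An overlap box shows the enter prompt, while the interaction input repossesses, offsets and detaches the driver.
; Autodrive selects a named Path actor and sets throttle once from Speed.
; Each tick it steers toward a look-ahead spline point, mapping yaw error to steering input.
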(event OnComponentBeginOverlap(DriverEnterBox)
  (params (OverlappedComponent :type Primitive%20Component%20Object%20Reference) (OtherActor :type Actor%20Object%20Reference) (OtherComp :type Primitive%20Component%20Object%20Reference) (OtherBodyIndex :type Integer) (bFromSweep :type Boolean) (SweepResult :type Hit%20Result%20Structure%20%28by%20ref%29))
  ;[0.15 0.15 0.15 0.5] Before Car Enter
  (bind _asbp_player (Utilities|Casting|CastToBP_Player OtherActor))
  (Rendering|SetVisibility (Variables|Default|GetEnterText) true false)
  (Variables|/Game/Dynamic/Character/BP_Player.BP_Player_C|SetVehicle _asbp_player 0)
  (Variables|Car|SetTryCarEnter true))

(event OnComponentEndOverlap(DriverEnterBox)
  (params (OverlappedComponent :type Primitive%20Component%20Object%20Reference) (OtherActor :type Actor%20Object%20Reference) (OtherComp :type Primitive%20Component%20Object%20Reference) (OtherBodyIndex :type Integer))
  ;[0.15 0.15 0.15 0.5] Cancel Enter
  (Rendering|SetVisibility (Variables|Default|GetEnterText) false false)
  (Variables|Car|SetTryCarEnter false))

(event Input|EnhancedActionEvents|EnhancedInputActionIA_CarInteraction
  (params (ActionValue :type Boolean) (ElapsedSeconds :type Float%20%28double-precision%29) (TriggeredSeconds :type Float%20%28double-precision%29) (InputAction :type Input%20Action%20Object%20Reference :default "/Game/Dynamic/Character/Input/Actions/IA_CarInteraction.IA_CarInteraction"))
  (bind _driver (Variables|Car|GetDriver))
  (bind _returnvalue (Transformation|GetActorLocation _driver))
  ;[0.15 0.15 0.15 0.5] Leave Car
  (Pawn|Possess (Game|GetPlayerController 0) _driver)
  ;[0.15 0.15 0.15 0.5] Change Player IMC (higher priority)
  (bind _asplayer_controller (Utilities|Casting|CastToPlayerController (Pawn|GetController _driver)))
  (Input|AddMappingContext (PlayerController|LocalPlayerSubsystems|GetEnhancedInputLocalPlayerSubsystem _asplayer_controller) "/Game/Dynamic/Character/Input/IMC_Default.IMC_Default" 10 "(bIgnoreAllPressedKeysUntilRelease=True,bForceImmediately=False,bNotifyUserSettings=False)")
  (Transformation|SetActorTransform _driver (Math|Transform|MakeTransform (Math|Vector|MakeVector (.x _returnvalue) (+ (.y _returnvalue) 3e+02) (.z _returnvalue)) "0, 0, 0" "1.000000,1.000000,1.000000"))
  (Collision|SetActorEnableCollision _driver true)
  (Transformation|DetachFromActor _driver "KeepWorld" "KeepWorld" "KeepWorld")
  (Variables|/Game/Dynamic/Character/BP_Player.BP_Player_C|SetInCar _driver false))

(event Input|EnhancedActionEvents|EnhancedInputActionIA_Camera
  (params (ActionValue :type Vector%202D%20Structure) (ElapsedSeconds :type Float%20%28double-precision%29) (TriggeredSeconds :type Float%20%28double-precision%29) (InputAction :type Input%20Action%20Object%20Reference :default "/Game/Dynamic/Vehicle/Input/Actions/IA_Camera.IA_Camera"))
  ;[0.15 0.15 0.15 0.5] Camera Movement w/ keyboard - QERF
  (Transformation|AddRelativeRotation (Variables|Default|GetSpringArm) (Math|Rotator|MakeRotator 0.0 (.y ActionValue) (.x ActionValue)) false false))

(event Input|EnhancedActionEvents|EnhancedInputActionIA_Throttle
  (params (ActionValue :type Float%20%28double-precision%29) (ElapsedSeconds :type Float%20%28double-precision%29) (TriggeredSeconds :type Float%20%28double-precision%29) (InputAction :type Input%20Action%20Object%20Reference :default "/Game/Dynamic/Vehicle/Input/Actions/IA_Throttle.IA_Throttle"))
  ;[0.15 0.15 0.15 0.5] Throttle input
  (Class|ChaosVehicleMovementComponent|SetThrottleInput (Variables|Default|GetVehicleMovementComponent) ActionValue))

(event Input|EnhancedActionEvents|EnhancedInputActionIA_Brake
  (params (ActionValue :type Float%20%28double-precision%29) (ElapsedSeconds :type Float%20%28double-precision%29) (TriggeredSeconds :type Float%20%28double-precision%29) (InputAction :type Input%20Action%20Object%20Reference :default "/Game/Dynamic/Vehicle/Input/Actions/IA_Brake.IA_Brake"))
  ;[0.15 0.15 0.15 0.5] Brake input
  (Class|ChaosVehicleMovementComponent|SetBrakeInput (Variables|Default|GetVehicleMovementComponent) ActionValue))

(event Input|EnhancedActionEvents|EnhancedInputActionIA_Steer
  (params (ActionValue :type Float%20%28double-precision%29) (ElapsedSeconds :type Float%20%28double-precision%29) (TriggeredSeconds :type Float%20%28double-precision%29) (InputAction :type Input%20Action%20Object%20Reference :default "/Game/Dynamic/Vehicle/Input/Actions/IA_Steer.IA_Steer"))
  ;[0.15 0.15 0.15 0.5] Steering input
  (Class|ChaosVehicleMovementComponent|SetSteeringInput (Variables|Default|GetVehicleMovementComponent) ActionValue))

(event Input|EnhancedActionEvents|EnhancedInputActionIA_Handbrake
  (params (ActionValue :type Boolean) (ElapsedSeconds :type Float%20%28double-precision%29) (TriggeredSeconds :type Float%20%28double-precision%29) (InputAction :type Input%20Action%20Object%20Reference :default "/Game/Dynamic/Vehicle/Input/Actions/IA_Handbrake.IA_Handbrake"))
  ;[0.15 0.15 0.15 0.5] Handbrake input
  (Class|ChaosVehicleMovementComponent|SetHandbrakeInput (Variables|Default|GetVehicleMovementComponent) ActionValue))

(event EventBeginPlay
  (bind _asplayer_controller (Utilities|Casting|CastToPlayerController (Pawn|GetController)))
  (Input|AddMappingContext (PlayerController|LocalPlayerSubsystems|GetEnhancedInputLocalPlayerSubsystem _asplayer_controller) "/Game/Dynamic/Vehicle/Input/IMC_Vehicle.IMC_Vehicle" 0 "(bIgnoreAllPressedKeysUntilRelease=True,bForceImmediately=False,bNotifyUserSettings=False)"))

(event EventTick
  (params (DeltaSeconds :type Float%20%28single-precision%29))
  ;[0.15 0.15 0.15 0.5] AutoDrive - Steering
  (if (Variables|AutoDrive|GetIsAuto)
    (bind _steering (CallFunction|GetPath))
    (Class|ChaosVehicleMovementComponent|SetSteeringInput (Variables|Default|GetVehicleMovementComponent) _steering)))

(event Input|MouseEvents|MouseX
  (params (AxisValue :type Float%20%28single-precision%29))
  ;[0.15 0.15 0.15 0.5] Camera Movement w/ mouse
  (Transformation|AddRelativeRotation (Variables|Default|GetSpringArm) (Math|Rotator|MakeRotator 0.0 0.0 AxisValue) false false))

(event Input|MouseEvents|MouseY
  (params (AxisValue :type Float%20%28single-precision%29))
  ;[0.15 0.15 0.15 0.5] Camera Movement w/ mouse
  (Transformation|AddRelativeRotation (Variables|Default|GetSpringArm) (Math|Rotator|MakeRotator 0.0 AxisValue 0.0) false false))

(event Input|EnhancedActionEvents|EnhancedInputActionIA_ActiveAutoDrive
  (params (ActionValue :type Boolean) (ElapsedSeconds :type Float%20%28double-precision%29) (TriggeredSeconds :type Float%20%28double-precision%29) (InputAction :type Input%20Action%20Object%20Reference :default "/Game/Dynamic/Vehicle/Input/Actions/IA_ActiveAutoDrive.IA_ActiveAutoDrive"))
  (if (Variables|AutoDrive|GetIsAuto)
    (Variables|AutoDrive|SetIsAuto false)
    (else
      (CallFunction|SelectPath)
      (Variables|AutoDrive|SetIsAuto true)
      (Class|ChaosVehicleMovementComponent|SetThrottleInput (Variables|Default|GetVehicleMovementComponent) (Variables|AutoDrive|GetSpeed)))))

(fn ConstructionScript)

(fn VehicleInputs
  (bind _vehiclemovementcomponent (Variables|Default|GetVehicleMovementComponent))
  (Class|ChaosVehicleMovementComponent|SetThrottleInput _vehiclemovementcomponent (Input|EnhancedActionValues|GetIA_Throttle))
  (Class|ChaosVehicleMovementComponent|SetBrakeInput _vehiclemovementcomponent (Input|EnhancedActionValues|GetIA_Brake))
  (Class|ChaosVehicleMovementComponent|SetSteeringInput _vehiclemovementcomponent (Input|EnhancedActionValues|GetIA_Steer))
  (Class|ChaosVehicleMovementComponent|SetHandbrakeInput _vehiclemovementcomponent (Input|EnhancedActionValues|GetIA_Handbrake)))

(fn GetPath
  (bind _returnvalue (Transformation|GetActorLocation))
  (bind _activepath (Variables|AutoDrive|GetActivePath))
  (bind _spline (Variables|/Game/Dynamic/Vehicle/Path.Path_C|GetSpline _activepath))
  (return (Math|Float|MapRangeClamped (.yaw (Math|Rotator|Delta(Rotator) (Math|Rotator|FindLookatRotation _returnvalue (Spline|FindLocationClosesttoWorldLocation _spline (+ (* (Math|Vector|Normalize (Class|SplineComponent|FindTangentClosesttoWorldLocation _spline _returnvalue "World")) 5e+02) _returnvalue) "World")) (Transformation|GetActorRotation))) -9e+01 9e+01 -1.0 1.0)))

(fn SelectPath
  (bind _outactors (Actor|GetAllActorsOfClass "/Game/Dynamic/Vehicle/Path.Path_C"))
  (for _array_element _outactors
    (if (== (Variables|/Game/Dynamic/Vehicle/Path.Path_C|GetName _array_element) (Variables|AutoDrive|GetPath))
      (Variables|AutoDrive|SetActivePath _array_element))))