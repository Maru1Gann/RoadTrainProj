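; Drivable Peterbilt 379 truck pawn with manual controls, an adjustable spring-arm camera, flip reset and toggleable autodrive.
; Autodrive finds a named Path actor, steers each tick toward a look-ahead spline point, brakes in sharp turns and stops at the end.
; A door trigger registers the truck with BP_Player, and exiting at low speed repossesses the driver.
; Docking and reset inputs message overlapping actors, intended as trailers, through Interact_Interface.
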(event OnComponentBeginOverlap(DriverEnterBox)
  (params (OverlappedComponent :type Primitive%20Component%20Object%20Reference) (OtherActor :type Actor%20Object%20Reference) (OtherComp :type Primitive%20Component%20Object%20Reference) (OtherBodyIndex :type Integer) (bFromSweep :type Boolean) (SweepResult :type Hit%20Result%20Structure%20%28by%20ref%29))
  ;[0.15 0.15 0.15 0.5] Before Car Enter
  (bind _asbp_player (Utilities|Casting|CastToBP_Player OtherActor))
  (Rendering|SetVisibility (Variables|Default|GetEnterText) true false)
  (Variables|/Game/Dynamic/Character/BP_Player.BP_Player_C|SetVehicle _asbp_player self)
  (Variables|Car|SetTryCarEnter true))

(event OnComponentEndOverlap(DriverEnterBox)
  (params (OverlappedComponent :type Primitive%20Component%20Object%20Reference) (OtherActor :type Actor%20Object%20Reference) (OtherComp :type Primitive%20Component%20Object%20Reference) (OtherBodyIndex :type Integer))
  ;[0.15 0.15 0.15 0.5] Cancel Enter
  (Rendering|SetVisibility (Variables|Default|GetEnterText) false false)
  (Variables|Car|SetTryCarEnter false))

(event Input|EnhancedActionEvents|EnhancedInputActionIA_CarInteraction
  (params (ActionValue :type Boolean) (ElapsedSeconds :type Float%20%28double-precision%29) (TriggeredSeconds :type Float%20%28double-precision%29) (InputAction :type Input%20Action%20Object%20Reference :default "/Game/Dynamic/Character/Input/Actions/IA_CarInteraction.IA_CarInteraction"))
  (bind _driver (Variables|Car|GetDriver))
  (bind _returnvalue (Pawn|GetController _driver))
  (bind _returnvalue_2 (Transformation|GetActorLocation _driver))
  ;[0.15 0.15 0.15 0.5] Leave Car
  (CallFunction|Stop)
  (if (<= (Class|ChaosVehicleMovementComponent|GetForwardSpeedMPH (Variables|Default|GetVehicleMovementComponent)) 5.0)
    (Pawn|Possess (Game|GetPlayerController 0) _driver)
    ;;[0.15 0.15 0.15 0.5] Change Player IMC (higher priority)
    (bind _asplayer_controller (Utilities|Casting|CastToPlayerController _returnvalue))
    (Class|EnhancedInputSubsystemInterface|ClearAllMappings(Message) (PlayerController|LocalPlayerSubsystems|GetEnhancedInputLocalPlayerSubsystem _asplayer_controller))
    (Input|AddMappingContext (PlayerController|LocalPlayerSubsystems|GetEnhancedInputLocalPlayerSubsystem _asplayer_controller) "/Game/Dynamic/Character/Input/IMC_Default.IMC_Default" 0 "(bIgnoreAllPressedKeysUntilRelease=True,bForceImmediately=False,bNotifyUserSettings=False)")
    ;;[0.15 0.15 0.15 0.5] Remove Vehicle UI
    (bind _asbp_player_controller_default (Utilities|Casting|CastToBP_PlayerController_Default _returnvalue))
    (Widget|RemovefromParent (Variables|/Game/Dynamic/BP_PlayerController_Default.BP_PlayerController_Default_C|GetVehicleUI_Ref _asbp_player_controller_default))
    (Variables|/Game/Dynamic/BP_PlayerController_Default.BP_PlayerController_Default_C|SetInCar _asbp_player_controller_default false)
    (Transformation|SetActorTransform _driver (Math|Transform|MakeTransform (Math|Vector|MakeVector (.x _returnvalue_2) (+ (.y _returnvalue_2) 3e+02) (.z _returnvalue_2)) "0, 0, 0" "1.000000,1.000000,1.000000"))
    (Collision|SetActorEnableCollision _driver true)
    (Transformation|DetachFromActor _driver "KeepWorld" "KeepWorld" "KeepWorld")
    (Variables|/Game/Dynamic/Character/BP_Player.BP_Player_C|SetInCar _driver false)))

(event Input|EnhancedActionEvents|EnhancedInputActionIA_CarRotationReset
  (params (ActionValue :type Boolean) (ElapsedSeconds :type Float%20%28double-precision%29) (TriggeredSeconds :type Float%20%28double-precision%29) (InputAction :type Input%20Action%20Object%20Reference :default "/Game/Dynamic/Vehicle/Input/Actions/IA_CarRotationReset.IA_CarRotationReset"))
  ;[0.15 0.15 0.15 0.5] Interact with BP using Blueprint Interface (Trailer)
  (CallFunction|CarReset)
  (bind _array_element (Utilities|Array|ForEachLoopwithBreak (Collision|GetOverlappingActors "/Script/Engine.Actor" :!class /Script/Engine.Actor) :!label _label)
    (:LoopBody
      (if (Utilities|DoesObjectImplementInterface _array_element "/Game/Dynamic/Vehicle/Truck_Trailer/Interact_Interface.Interact_Interface_C")
        (Class|InteractInterface|InteractReset(Message) _array_element self)
        (goto _label Break)))))

(event Input|EnhancedActionEvents|EnhancedInputActionIA_Throttle
  (params (ActionValue :type Float%20%28double-precision%29) (ElapsedSeconds :type Float%20%28double-precision%29) (TriggeredSeconds :type Float%20%28double-precision%29) (InputAction :type Input%20Action%20Object%20Reference :default "/Game/Dynamic/Vehicle/Input/Actions/IA_Throttle.IA_Throttle"))
  ;[0.15 0.15 0.15 0.5] Throttle input
  (if (not (Variables|Auto|GetIsAuto))
    (Class|ChaosVehicleMovementComponent|SetThrottleInput (Variables|Default|GetVehicleMovementComponent) ActionValue)))

(event Input|EnhancedActionEvents|EnhancedInputActionIA_Brake
  (params (ActionValue :type Float%20%28double-precision%29) (ElapsedSeconds :type Float%20%28double-precision%29) (TriggeredSeconds :type Float%20%28double-precision%29) (InputAction :type Input%20Action%20Object%20Reference :default "/Game/Dynamic/Vehicle/Input/Actions/IA_Brake.IA_Brake"))
  ;[0.15 0.15 0.15 0.5] Brake input
  (Class|ChaosVehicleMovementComponent|SetBrakeInput (Variables|Default|GetVehicleMovementComponent) ActionValue))

(event Input|EnhancedActionEvents|EnhancedInputActionIA_Docking
  (params (ActionValue :type Boolean) (ElapsedSeconds :type Float%20%28double-precision%29) (TriggeredSeconds :type Float%20%28double-precision%29) (InputAction :type Input%20Action%20Object%20Reference :default "/Game/Dynamic/Vehicle/Input/Actions/IA_Docking.IA_Docking"))
  ;[0.15 0.15 0.15 0.5] Interact with BP using Blueprint Interface (Trailer)
  (bind _array_element (Utilities|Array|ForEachLoopwithBreak (Collision|GetOverlappingActors "/Script/Engine.Actor" :!class /Script/Engine.Actor) :!label _label)
    (:LoopBody
      (if (Utilities|DoesObjectImplementInterface _array_element "/Game/Dynamic/Vehicle/Truck_Trailer/Interact_Interface.Interact_Interface_C")
        (Class|InteractInterface|Interact(Message) _array_element self)
        (goto _label Break)))))

(event Input|EnhancedActionEvents|EnhancedInputActionIA_Steer
  (params (ActionValue :type Float%20%28double-precision%29) (ElapsedSeconds :type Float%20%28double-precision%29) (TriggeredSeconds :type Float%20%28double-precision%29) (InputAction :type Input%20Action%20Object%20Reference :default "/Game/Dynamic/Vehicle/Input/Actions/IA_Steer.IA_Steer"))
  ;[0.15 0.15 0.15 0.5] Steering input
  (Class|ChaosVehicleMovementComponent|SetSteeringInput (Variables|Default|GetVehicleMovementComponent) ActionValue))

(event Input|EnhancedActionEvents|EnhancedInputActionIA_Handbrake
  (params (ActionValue :type Boolean) (ElapsedSeconds :type Float%20%28double-precision%29) (TriggeredSeconds :type Float%20%28double-precision%29) (InputAction :type Input%20Action%20Object%20Reference :default "/Game/Dynamic/Vehicle/Input/Actions/IA_Handbrake.IA_Handbrake"))
  ;[0.15 0.15 0.15 0.5] Handbrake input
  (Class|ChaosVehicleMovementComponent|SetHandbrakeInput (Variables|Default|GetVehicleMovementComponent) ActionValue))

(event Input|EnhancedActionEvents|EnhancedInputActionIA_CameraReset
  (params (ActionValue :type Boolean) (ElapsedSeconds :type Float%20%28double-precision%29) (TriggeredSeconds :type Float%20%28double-precision%29) (InputAction :type Input%20Action%20Object%20Reference :default "/Game/Dynamic/Vehicle/Input/Actions/IA_CameraReset.IA_CameraReset"))
  ;[0.15 0.15 0.15 0.5] Camera Movement w/ mouse
  ;;[0.15 0.15 0.15 0.5] Default value
  (Transformation|SetRelativeLocation (Variables|Default|GetSpringArm_x) "0.000000,0.000000,400.000000" false false)
  (Transformation|SetRelativeRotation (Variables|Default|GetSpringArm) (Math|Rotator|MakeRotator 0.0 -1e+01 0.0) false false))

(event EventBeginPlay
  (bind _asplayer_controller (Utilities|Casting|CastToPlayerController (Pawn|GetController)))
  (Input|AddMappingContext (PlayerController|LocalPlayerSubsystems|GetEnhancedInputLocalPlayerSubsystem _asplayer_controller) "/Game/Dynamic/Vehicle/Input/IMC_Vehicle.IMC_Vehicle" 10 "(bIgnoreAllPressedKeysUntilRelease=True,bForceImmediately=False,bNotifyUserSettings=False)"))

(event Collision|EventActorBeginOverlap
  (params (OtherActor :type Actor%20Object%20Reference)))

(event Input|MouseEvents|MouseX
  (params (AxisValue :type Float%20%28single-precision%29))
  (bind _springarm (Variables|Default|GetSpringArm))
  (bind _relativerotation (Variables|/Script/Engine.SceneComponent|GetRelativeRotation _springarm))
  (bind _returnvalue (Math|Float|Clamp(Float) (.yaw _relativerotation) -1.8e+02 1.8e+02))
  ;[0.15 0.15 0.15 0.5] Camera Movement w/ mouse
  (Transformation|SetRelativeRotation _springarm (Math|Rotator|MakeRotator 0.0 (Math|Float|Clamp(Float) (.pitch _relativerotation) -8e+01 2e+01) _returnvalue) false false)
  ;;[0.15 0.15 0.15 0.5] Camera Shift when Shift key is clicked
  (if (Input|EnhancedActionValues|GetIA_Camera_Shift)
    (Transformation|AddLocalOffset (Variables|Default|GetSpringArm_x) (Math|Vector|MakeVector (* (Math|Float|MapRangeClamped (Math|Conversions|ToFloat(Boolean) (and (< _returnvalue 9e+01) (> _returnvalue -9e+01))) 0.0 1.0 -1e+01 1e+01) (stale Input|MouseEvents|MouseY AxisValue)) 0.0 0.0) false false)
    (else
      (Transformation|AddRelativeRotation _springarm (Math|Rotator|MakeRotator 0.0 (stale Input|MouseEvents|MouseY AxisValue) AxisValue) false false))))

(event Input|MouseEvents|MouseY
  (params (AxisValue :type Float%20%28single-precision%29))
  (bind _springarm (Variables|Default|GetSpringArm))
  (bind _relativerotation (Variables|/Script/Engine.SceneComponent|GetRelativeRotation _springarm))
  (bind _returnvalue (Math|Float|Clamp(Float) (.yaw _relativerotation) -1.8e+02 1.8e+02))
  ;[0.15 0.15 0.15 0.5] Camera Movement w/ mouse
  (Transformation|SetRelativeRotation _springarm (Math|Rotator|MakeRotator 0.0 (Math|Float|Clamp(Float) (.pitch _relativerotation) -8e+01 2e+01) _returnvalue) false false)
  ;;[0.15 0.15 0.15 0.5] Camera Shift when Shift key is clicked
  (if (Input|EnhancedActionValues|GetIA_Camera_Shift)
    (Transformation|AddLocalOffset (Variables|Default|GetSpringArm_x) (Math|Vector|MakeVector (* (Math|Float|MapRangeClamped (Math|Conversions|ToFloat(Boolean) (and (< _returnvalue 9e+01) (> _returnvalue -9e+01))) 0.0 1.0 -1e+01 1e+01) AxisValue) 0.0 0.0) false false)
    (else
      (Transformation|AddRelativeRotation _springarm (Math|Rotator|MakeRotator 0.0 AxisValue (stale Input|MouseEvents|MouseX AxisValue)) false false))))

(event Input|EnhancedActionEvents|EnhancedInputActionIA_ActiveAutoDrive
  (params (ActionValue :type Boolean) (ElapsedSeconds :type Float%20%28double-precision%29) (TriggeredSeconds :type Float%20%28double-precision%29) (InputAction :type Input%20Action%20Object%20Reference :default "/Game/Dynamic/Vehicle/Input/Actions/IA_ActiveAutoDrive.IA_ActiveAutoDrive"))
  ;[0.15 0.15 0.15 0.5] Throttle
  (if (Variables|Auto|GetIsAuto)
    ;[0.15 0.15 0.15 0.5] Not Auto
    (Variables|Auto|SetIsAuto false)
    (CallFunction|VehicleInputs)
    (else
      (CallFunction|SelectPath)
      (Variables|Auto|SetIsAuto true)
      (Class|ChaosVehicleMovementComponent|SetThrottleInput (Variables|Default|GetVehicleMovementComponent) (Variables|Auto|GetSpeed)))))

(event EventTick
  (params (DeltaSeconds :type Float%20%28single-precision%29))
  (bind _activepath (Variables|Auto|GetActivePath))
  (bind _vehiclemovementcomponent (Variables|Default|GetVehicleMovementComponent))
  (bind _spline (Variables|/Game/Dynamic/Vehicle/Path.Path_C|GetSpline _activepath))
  ;[0.15 0.15 0.15 0.5] AutoDrive - Steering
  (if (Variables|Auto|GetIsAuto)
    (bind _steering (CallFunction|GetPath))
    (if (Math|Float|NearlyEqual(Float) (Class|SplineComponent|GetDistanceAlongSplineatLocation _spline (Transformation|GetActorLocation) "World") (Spline|GetSplineLength _spline) 1e+02)
      (CallFunction|Stop)
      (else
        (Class|ChaosVehicleMovementComponent|SetSteeringInput _vehiclemovementcomponent _steering)
        (if (> (Math|Float|Absolute(Float) _steering) 0.5)
          (Development|PrintString (Utilities|String|ToString(Float) (Math|Float|Clamp(Float) (Math|Float|Absolute(Float) _steering) 0.0 0.2)))
          (Class|ChaosVehicleMovementComponent|SetBrakeInput _vehiclemovementcomponent (Math|Float|Clamp(Float) (Math|Float|Absolute(Float) _steering) 0.0 0.2))
          (Utilities|FlowControl|Delay 1.0)
          (Class|ChaosVehicleMovementComponent|SetBrakeInput _vehiclemovementcomponent 0.0))))
    (else
      ;[0.15 0.15 0.15 0.5] Not Auto
      (CallFunction|VehicleInputs))))

(fn ConstructionScript)

(fn VehicleInputs
  (bind _vehiclemovementcomponent (Variables|Default|GetVehicleMovementComponent))
  (Class|ChaosVehicleMovementComponent|SetThrottleInput _vehiclemovementcomponent (Input|EnhancedActionValues|GetIA_Throttle))
  (Class|ChaosVehicleMovementComponent|SetBrakeInput _vehiclemovementcomponent (Input|EnhancedActionValues|GetIA_Brake))
  (Class|ChaosVehicleMovementComponent|SetSteeringInput _vehiclemovementcomponent (Input|EnhancedActionValues|GetIA_Steer))
  (Class|ChaosVehicleMovementComponent|SetHandbrakeInput _vehiclemovementcomponent (Input|EnhancedActionValues|GetIA_Handbrake)))

(fn GetPath
  (bind _returnvalue (Transformation|GetActorLocation))
  (bind _activepath (Variables|Auto|GetActivePath))
  (bind _spline (Variables|/Game/Dynamic/Vehicle/Path.Path_C|GetSpline _activepath))
  (return (Math|Float|MapRangeClamped (.yaw (Math|Rotator|Delta(Rotator) (Math|Rotator|FindLookatRotation _returnvalue (Spline|FindLocationClosesttoWorldLocation _spline (+ (* (Math|Vector|Normalize (Class|SplineComponent|FindTangentClosesttoWorldLocation _spline _returnvalue "World")) 1.5e+02) _returnvalue) "World")) (Transformation|GetActorRotation))) -9e+01 9e+01 -1.0 1.0)))

(fn SelectPath
  (bind _outactors (Actor|GetAllActorsOfClass "/Game/Dynamic/Vehicle/Path.Path_C"))
  (for _array_element _outactors
    (if (== (Variables|/Game/Dynamic/Vehicle/Path.Path_C|GetName _array_element) (Variables|Auto|GetPath))
      (Variables|Auto|SetActivePath _array_element))))

(fn Stop
  (bind _vehiclemovementcomponent (Variables|Default|GetVehicleMovementComponent))
  (Class|ChaosVehicleMovementComponent|SetThrottleInput _vehiclemovementcomponent 0.0)
  (Class|ChaosVehicleMovementComponent|SetHandbrakeInput _vehiclemovementcomponent true)
  (return))

(fn CarReset
  (bind _mesh (Variables|Character|GetMesh))
  (Physics|SetPhysicsLinearVelocity _mesh "0, 0, 0" false "None")
  (Class|PrimitiveComponent|SetPhysicsAngularVelocityinDegrees _mesh "0, 0, 0" false "None")
  (Transformation|SetActorRotation "0, 0, 0" true)
  (Transformation|AddWorldOffset (Variables|Character|GetMesh) "0.000000,0.000000,400.000000" false true))