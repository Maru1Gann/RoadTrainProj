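; Drivable-truck trailer that couples to and uncouples from a BP_Peterbilt379_3 tractor.
; While the truck overlaps the trigger, a 0.1-second delay loop checks DockingArea alignment, caches the snap offset and toggles the dock prompt.
; Interact flip-flops between snapping and constraining the trailer to the truck body, and breaking the constraint, switching mesh constraint mode and throttle input.
; InteractReset uprights the trailer, teleports it above the docking point and reattaches it.
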(event OnComponentBeginOverlap(Trigger)
  (params (OverlappedComponent :type Primitive%20Component%20Object%20Reference) (OtherActor :type Actor%20Object%20Reference) (OtherComp :type Primitive%20Component%20Object%20Reference) (OtherBodyIndex :type Integer) (bFromSweep :type Boolean) (SweepResult :type Hit%20Result%20Structure%20%28by%20ref%29))
  (bind _trigger (Variables|Default|GetTrigger))
  (bind _returnvalue (Transformation|GetWorldLocation _trigger))
  (Variables|Default|SetTryDock true)
  (bind _asbp_peterbilt_379_3 (Utilities|Casting|CastToBP_Peterbilt379_3 OtherActor :!label _label))
  (bind _output_get (Variables|Default|SetCanDock (Utilities|Operators|EqualEqual (Transformation|GetWorldLocation (Variables|/Game/Dynamic/Vehicle/peterbilt-379/BP_Peterbilt379_3.BP_Peterbilt379_3_C|GetDockingArea _asbp_peterbilt_379_3)) _returnvalue 1e+02)))
  (Variables|Default|SetdockingLocation (Math|Vector|MakeVector (.x (- (Transformation|GetWorldLocation (Variables|/Game/Dynamic/Vehicle/peterbilt-379/BP_Peterbilt379_3.BP_Peterbilt379_3_C|GetDockingArea _asbp_peterbilt_379_3)) _returnvalue)) (.y (- (Transformation|GetWorldLocation (Variables|/Game/Dynamic/Vehicle/peterbilt-379/BP_Peterbilt379_3.BP_Peterbilt379_3_C|GetDockingArea _asbp_peterbilt_379_3)) _returnvalue)) 0.0))
  (Rendering|SetVisibility (Variables|Default|GetDockText) _output_get false)
  (Utilities|FlowControl|Delay 0.1)
  (if (Variables|Default|GetTryDock)
    (goto _label)))

(event OnComponentEndOverlap(Trigger)
  (params (OverlappedComponent :type Primitive%20Component%20Object%20Reference) (OtherActor :type Actor%20Object%20Reference) (OtherComp :type Primitive%20Component%20Object%20Reference) (OtherBodyIndex :type Integer))
  (Utilities|Casting|CastToBP_Peterbilt379_3 OtherActor)
  (Variables|Default|SetTryDock false)
  (Rendering|SetVisibility (Variables|Default|GetDockText) false false))

(event EventInteractReset
  (params (Trackor :type BP%20Peterbilt%20379%203%20Object%20Reference))
  (bind _mesh (Variables|Character|GetMesh))
  (bind _trigger (Variables|Default|GetTrigger))
  (bind _dockingarea (Variables|/Game/Dynamic/Vehicle/peterbilt-379/BP_Peterbilt379_3.BP_Peterbilt379_3_C|GetDockingArea Trackor))
  (bind _physicsconstraint (Variables|Default|GetPhysicsConstraint))
  (bind _returnvalue (Transformation|GetWorldLocation _dockingarea))
  (bind _returnvalue_2 (Transformation|GetWorldLocation _trigger))
  (bind _returnvalue_3 (- _returnvalue _returnvalue_2))
  ;[0.15 0.15 0.15 0.5] Reset
  (Class|PhysicsConstraintComponent|BreakConstraint _physicsconstraint)
  (Class|PrimitiveComponent|SetConstraintMode _mesh "Default")
  (Transformation|SetActorRotation "0, 0, 0" true)
  (Transformation|AddWorldOffset _mesh (Math|Vector|MakeVector (.x _returnvalue_3) (.y _returnvalue_3) 4e+02) false true)
  (Class|PhysicsConstraintComponent|SetConstrainedComponents _physicsconstraint (Variables|/Script/ChaosVehicles.WheeledVehiclePawn|GetMesh Trackor) "body" _mesh "Truck_Trailer")
  (Class|PrimitiveComponent|SetConstraintMode _mesh "None"))

(event EventInteract
  (params (Trackor :type BP%20Peterbilt%20379%203%20Object%20Reference))
  (bind _vehiclemovementcomponent (Variables|Default|GetVehicleMovementComponent))
  (bind _physicsconstraint (Variables|Default|GetPhysicsConstraint))
  (bind _mesh (Variables|Character|GetMesh))
  (if (Variables|Default|GetCanDock)
    (Utilities|FlowControl|FlipFlop
      (:A
        (Transformation|AddWorldOffset _mesh (Variables|Default|GetdockingLocation) false true)
        (Class|ChaosVehicleMovementComponent|SetThrottleInput _vehiclemovementcomponent 0.01)
        (Class|PhysicsConstraintComponent|SetConstrainedComponents _physicsconstraint (Variables|/Script/ChaosVehicles.WheeledVehiclePawn|GetMesh Trackor) "body" _mesh "Truck_Trailer")
        (Class|PrimitiveComponent|SetConstraintMode (Variables|Character|GetMesh) "None")
        (Variables|Default|SetTryDock false))
      (:B
        (Class|ChaosVehicleMovementComponent|SetThrottleInput _vehiclemovementcomponent 0.0)
        (Class|PhysicsConstraintComponent|BreakConstraint _physicsconstraint)
        (Class|PrimitiveComponent|SetConstraintMode (Variables|Character|GetMesh) "Default")
        (Variables|Default|SetTryDock true)))
    (Rendering|SetVisibility (Variables|Default|GetDockText) (Variables|Default|GetTryDock) false)))

(fn ConstructionScript)