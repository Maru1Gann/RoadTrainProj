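; Player controller that owns the root HUD for truck driving and on-foot play, and opens the pause UI on Escape.
; BeginPlay branches on game mode to cache the truck or character, with intro dialogue preceding the vehicle HUD on a first drive game.
; Tick feeds truck speed, gear, distance and heading to the HUD while driving.
; View-change and drive events swap the HUD for a dialogue widget, whose back button restores it and, outside drive events, the truck camera.
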(event Custom|OnDialogueFinished
  (bind _rootui (Variables|UI|GetRootUI))
  (Widget|RemovefromParent (Variables|UI|GetDialogueUI))
  (UserInterface|Viewport|AddtoViewport _rootui 0)
  (Class|WidgetSwitcher|SetActiveWidgetIndex (Variables|/Game/Dynamic/UI/WBP_RootUI.WBP_RootUI_C|GetWidgetSwitcher_Pawn _rootui) 1)
  (Input|SetInputModeGameandUI (Game|GetPlayerController 0) 0 "DoNotLock" false false))

(event Custom|ChangeViewEvent
  (params (Selection :type Enum_TrailerCam%20Enum :default "NewEnumerator3"))
  ;[0.15 0.15 0.15 0.5] 3D Widget Interaction
  (bind _output_get (CallFunction|GetTrailerRef))
  (Default|SetViewTargetCameraTransform _output_get Selection)
  (Widget|SetVisibility (Variables|UI|GetRootUI) "Hidden")
  (bind _returnvalue (UserInterface|CreateWidget "/Game/Dynamic/UI/WBP_DialogueTest.WBP_DialogueTest_C"))
  (UserInterface|Viewport|AddtoViewport _returnvalue 0)
  (Input|SetInputModeUIOnly (Game|GetPlayerController 0) 0 "DoNotLock" false)
  (EventDispatchers|BindEventtoOnBackButtonClicked _returnvalue (delegate Custom|ChangeToMainCamEvent)))

(event Custom|ChangeToMainCamEvent
  ;[0.15 0.15 0.15 0.5] 3D Widget Interaction
  (Widget|RemovefromParent (stale Custom|ChangeViewEvent _returnvalue))
  (Widget|SetVisibility (Variables|UI|GetRootUI) "SelfHitTestInvisible")
  (Input|SetInputModeGameandUI (Game|GetPlayerController 0) 0 "DoNotLock" false false)
  (if (Variables|Default|GetIsDriveEvent)
    (Variables|Default|SetIsDriveEvent false)
    (else
      (Default|SetViewTargetCamera (Variables|Vehicle|GetTruck_Ref))))
  (Default|CallOnBacktoMainCam))

(event Custom|DriveEvent
  ;[0.15 0.15 0.15 0.5] 3D Widget Interaction
  (Variables|Default|SetIsDriveEvent true)
  (Widget|SetVisibility (Variables|UI|GetRootUI) "Hidden")
  (bind _returnvalue (UserInterface|CreateWidget "/Game/Dynamic/UI/WBP_DialogueTest.WBP_DialogueTest_C"))
  (UserInterface|Viewport|AddtoViewport _returnvalue 0)
  (Input|SetInputModeUIOnly (Game|GetPlayerController 0) 0 "DoNotLock" false)
  (EventDispatchers|BindEventtoOnBackButtonClicked _returnvalue (delegate Custom|ChangeToMainCamEvent)))

(event EventBeginPlay
  (Variables|Default|SetbShowMouseCursor true)
  (Utilities|Casting|CastToGM_DriveMode (Game|GetGameMode)
    (:then
      (Variables|Default|SetIsDirveGM true)
      (bind _asbp_peterbilt_379_3 (Utilities|Casting|CastToBP_Peterbilt379_3 (Game|Player|GetPlayerPawn 0)))
      (Variables|Vehicle|SetTruck_Ref _asbp_peterbilt_379_3)
      (bind _returnvalue (UserInterface|CreateWidget "/Game/Dynamic/UI/WBP_RootUI.WBP_RootUI_C"))
      (Variables|UI|SetRootUI _returnvalue)
      (if (Variables|Default|GetIsFirstGame)
        (bind _returnvalue_2 (UserInterface|CreateWidget "/Game/Dynamic/UI/DialogueUI/WBP_Dialogue.WBP_Dialogue_C"))
        (bind _output_get (Variables|UI|SetDialogueUI _returnvalue_2))
        (UserInterface|Viewport|AddtoViewport _output_get 10)
        (Input|SetInputModeUIOnly (Game|GetPlayerController 0) _output_get "DoNotLock" false)
        (EventDispatchers|BindEventtoOnDialogueFinished _output_get (delegate Custom|OnDialogueFinished))
        (else
          (UserInterface|Viewport|AddtoViewport (Variables|UI|GetRootUI) 0)
          (Class|WidgetSwitcher|SetActiveWidgetIndex (Variables|/Game/Dynamic/UI/WBP_RootUI.WBP_RootUI_C|GetWidgetSwitcher_Pawn (Variables|UI|GetRootUI)) 1)
          (Input|SetInputModeGameandUI (Game|GetPlayerController 0) 0 "DoNotLock" false false))))
    (:CastFailed
      (bind _returnvalue_3 (UserInterface|CreateWidget "/Game/Dynamic/UI/WBP_RootUI.WBP_RootUI_C"))
      (bind _output_get_2 (Variables|UI|SetRootUI _returnvalue_3))
      (UserInterface|Viewport|AddtoViewport _output_get_2 0)
      (bind _asbp_player (Utilities|Casting|CastToBP_Player (Game|Player|GetPlayerPawn 0)))
      (Variables|Default|SetCharacter_Ref _asbp_player))))

(event EventTick
  (params (DeltaSeconds :type Float%20%28single-precision%29))
  (bind _truck_ref (Variables|Vehicle|GetTruck_Ref))
  (bind _rootui (Variables|UI|GetRootUI))
  (bind _vehiclemovementcomponent (Variables|/Script/ChaosVehicles.WheeledVehiclePawn|GetVehicleMovementComponent _truck_ref))
  (if (Variables|Default|GetIsDirveGM)
    ;[0.15 0.15 0.15 0.5] 차량 주행 중에만 사용
    (Default|UpdateSpeed _rootui (Vehicle|GetForwardSpeed _vehiclemovementcomponent) :!label _label)
    (Default|UpdateGear _rootui (Class|ChaosVehicleMovementComponent|GetCurrentGear _vehiclemovementcomponent))
    (bind _totaldistance (Default|GetTotalDistanceKm (Variables|Vehicle|GetTruck_Ref)))
    (Default|UpdateTotalDistance _rootui _totaldistance)
    (Default|UpdateCompass _rootui (- 3.6e+02 (.yaw (Transformation|GetActorRotation (Variables|Vehicle|GetTruck_Ref)))))
    (elif (Variables|/Game/Dynamic/Character/BP_Player.BP_Player_C|GetInCar (Variables|Default|GetCharacter_Ref))
      (goto _label))))

(event Input|KeyboardEvents|Escape
  (params (Key :type Key%20Structure))
  (:Pressed
    (Default|CallPasueUI (Variables|UI|GetRootUI))))

(fn ConstructionScript)

(fn ShowVehicleUI
  (Class|WidgetSwitcher|SetActiveWidgetIndex (Variables|/Game/Dynamic/UI/WBP_RootUI.WBP_RootUI_C|GetWidgetSwitcher_Pawn (Variables|UI|GetRootUI)) 1)
  (bind _asbp_peterbilt_379_3 (Utilities|Casting|CastToBP_Peterbilt379_3 (Game|Player|GetPlayerPawn 0)))
  (Variables|Vehicle|SetTruck_Ref _asbp_peterbilt_379_3))

(fn ShowCharacterUI
  (Class|WidgetSwitcher|SetActiveWidgetIndex (Variables|/Game/Dynamic/UI/WBP_RootUI.WBP_RootUI_C|GetWidgetSwitcher_Pawn (Variables|UI|GetRootUI))))

(fn GetTrailerRef
  (Utilities|IsValid (Variables|Vehicle|GetTrailer_Ref)
    (:Is%20Valid
      (return (Variables|Vehicle|GetTrailer_Ref)))
    (:Is%20Not%20Valid
      (bind _returnvalue (Actor|GetActorOfClass "/Game/Dynamic/Vehicle/Truck_Trailer/BP_Truck_Trailer.BP_Truck_Trailer_C"))
      (Utilities|IsValid _returnvalue
        (:Is%20Valid
          (Variables|Vehicle|SetTrailer_Ref _returnvalue)
          (return (Variables|Vehicle|GetTrailer_Ref)))
        (:Is%20Not%20Valid
          (Development|PrintString "Fail"))))))