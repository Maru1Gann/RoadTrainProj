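; BP_Player is the on-foot player that moves with Enhanced Input and can board a truck as its driver.
; BeginPlay caches the BP_Peterbilt379_3 found in the level and adds the default mapping context.
; Move input applies world-axis movement.
; When TryCarEnter allows it, interaction possesses the truck, swaps to vehicle input and UI, disables the character's collision and attaches it to the Driver_Seat socket.
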(event Input|EnhancedActionEvents|EnhancedInputActionIA_Move
  (params (ActionValue :type Vector%202D%20Structure) (ElapsedSeconds :type Float%20%28double-precision%29) (TriggeredSeconds :type Float%20%28double-precision%29) (InputAction :type Input%20Action%20Object%20Reference :default "/Game/Dynamic/Character/Input/Actions/IA_Move.IA_Move"))
  ;[0.15 0.15 0.15 0.5] Move
  (Pawn|Input|AddMovementInput (Math|Conversions|ToVector(Vector2D) ActionValue) 1.0 false))

(event Input|EnhancedActionEvents|EnhancedInputActionIA_CarInteraction
  (params (ActionValue :type Boolean) (ElapsedSeconds :type Float%20%28double-precision%29) (TriggeredSeconds :type Float%20%28double-precision%29) (InputAction :type Input%20Action%20Object%20Reference :default "/Game/Dynamic/Character/Input/Actions/IA_CarInteraction.IA_CarInteraction"))
  (bind _self self)
  (bind _vehicle (Variables|Default|GetVehicle))
  (bind _returnvalue (Pawn|GetController _vehicle))
  ;[0.15 0.15 0.15 0.5] Enter Car
  (if (Variables|/Game/Dynamic/Vehicle/peterbilt-379/BP_Peterbilt379_3.BP_Peterbilt379_3_C|GetTryCarEnter _vehicle)
    (Variables|/Game/Dynamic/Vehicle/peterbilt-379/BP_Peterbilt379_3.BP_Peterbilt379_3_C|SetDriver _vehicle _self)
    (Pawn|Possess (Game|GetPlayerController 0) _vehicle)
    ;[0.15 0.15 0.15 0.5] Vehicle Control
    (bind _asplayer_controller (Utilities|Casting|CastToPlayerController _returnvalue))
    (Class|EnhancedInputSubsystemInterface|ClearAllMappings(Message) (PlayerController|LocalPlayerSubsystems|GetEnhancedInputLocalPlayerSubsystem _asplayer_controller))
    (Input|AddMappingContext (PlayerController|LocalPlayerSubsystems|GetEnhancedInputLocalPlayerSubsystem _asplayer_controller) "/Game/Dynamic/Vehicle/Input/IMC_Vehicle.IMC_Vehicle" 10 "(bIgnoreAllPressedKeysUntilRelease=True,bForceImmediately=False,bNotifyUserSettings=False)")
    ;[0.15 0.15 0.15 0.5] Add Vehicle UI
    (bind _asbp_player_controller_default (Utilities|Casting|CastToBP_PlayerController_Default _returnvalue))
    (Default|ShowVehicleUI _asbp_player_controller_default)
    (Collision|SetActorEnableCollision _self false)
    (Transformation|AttachActorToActor _vehicle "Driver_Seat" "SnapToTarget" "SnapToTarget" "KeepWorld" true)
    (Variables|Default|SetInCar true)))

(event EventBeginPlay
  (|CallParentFunction)
  (bind _returnvalue (Actor|GetActorOfClass "/Game/Dynamic/Vehicle/peterbilt-379/BP_Peterbilt379_3.BP_Peterbilt379_3_C"))
  (Variables|Default|SetVehicle _returnvalue)
  (bind _asplayer_controller (Utilities|Casting|CastToPlayerController (Pawn|GetController)))
  (Input|AddMappingContext (PlayerController|LocalPlayerSubsystems|GetEnhancedInputLocalPlayerSubsystem _asplayer_controller) "/Game/Dynamic/Character/Input/IMC_Default.IMC_Default" 0 "(bIgnoreAllPressedKeysUntilRelease=True,bForceImmediately=False,bNotifyUserSettings=False)"))

(event Collision|EventActorBeginOverlap
  (params (OtherActor :type Actor%20Object%20Reference))
  (|CallParentFunction OtherActor) ; This node is disabled and will not be called.\nDrag off pins to build functionality.
)

(event EventTick
  (params (DeltaSeconds :type Float%20%28single-precision%29))
  (|CallParentFunction DeltaSeconds) ; This node is disabled and will not be called.\nDrag off pins to build functionality.
)

(fn ConstructionScript
  (|CallParentFunction))